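; DayNight_BP is an interactable mesh actor that toggles between day and night looks through a material parameter.
; Its construction script creates a dynamic material instance on the mesh, and a box overlap enables or disables player 0 input on the actor.
; The DefualtAction input reads NightValue and plays or reverses the GoNight timeline, which drives that parameter for a gradual transition.
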(event OnComponentBeginOverlap(Box)
  (params (OtherActor :type Actor%20Object%20Reference) (OtherComp :type Primitive%20Component%20Object%20Reference) (OtherBodyIndex :type Integer) (bFromSweep :type Boolean) (SweepResult :type Hit%20Result%20Structure%20%28by%20ref%29))
  (Input|EnableInput (Game|GetPlayerController 0)))

(event OnComponentEndOverlap(Box)
  (params (OtherActor :type Actor%20Object%20Reference) (OtherComp :type Primitive%20Component%20Object%20Reference) (OtherBodyIndex :type Integer))
  (Input|DisableInput (Game|GetPlayerController 0)))

(event EventBeginPlay)

(event Collision|EventActorBeginOverlap
  (params (OtherActor :type Actor%20Object%20Reference)))

(event EventTick
  (params (DeltaSeconds :type Float%20%28single-precision%29)))

(event Input|ActionEvents|InputActionDefualtAction
  (params (Key :type Key%20Structure :default "AnyKey"))
  (:Pressed
    (bind _returnvalue (Rendering|Material|GetScalarParameterValue (Variables|Default|GetMaterialDynamic) "NightValue" :!class /Script/Engine.MaterialInstanceDynamic))
    (if (> _returnvalue 0.5)
      (bind _gonight (Timeline|GoNight Reverse)
        (:Update
          (Rendering|Material|SetScalarParameterValue (Variables|Default|GetMaterialDynamic) "NightValue" _gonight :!class /Script/Engine.MaterialInstanceDynamic)))
      (else
        (Timeline|GoNight Play)))))

(fn ConstructionScript
  (bind _returnvalue (Rendering|Material|CreateDynamicMaterialInstance (Variables|/Script/Engine.StaticMeshActor|GetStaticMeshComponent (Variables|Default|GetMesh)) 0 0 :!class /Script/Engine.PrimitiveComponent))
  (Variables|Default|SetMaterialDynamic _returnvalue))