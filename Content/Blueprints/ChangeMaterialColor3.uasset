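; An interactive trigger actor that lets the player cycle the color of a set of referenced meshes while inside its box.
; The construction script creates a dynamic material instance for each mesh.
; Box overlaps toggle player input; ChangeColors applies the current Colors entry to every instance's "Color" parameter, then advances the index.
; The wrap check lets the index reach the array length, one past the last color, before resetting.
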(event OnComponentBeginOverlap(Box)
  (params (OtherActor :type Actor%20Object%20Reference) (OtherComp :type Primitive%20Component%20Object%20Reference) (OtherBodyIndex :type Integer) (bFromSweep :type Boolean) (SweepResult :type Hit%20Result%20Structure%20%28by%20ref%29))
  (Input|EnableInput (Game|GetPlayerController 0)))

(event OnComponentEndOverlap(Box)
  (params (OtherActor :type Actor%20Object%20Reference) (OtherComp :type Primitive%20Component%20Object%20Reference) (OtherBodyIndex :type Integer))
  (Input|DisableInput (Game|GetPlayerController 0)))

(event EventBeginPlay)

(event Collision|EventActorBeginOverlap
  (params (OtherActor :type Actor%20Object%20Reference)))

(event EventTick
  (params (DeltaSeconds :type Float%20%28single-precision%29)))

(event Input|ActionEvents|InputActionChangeColors
  (params (Key :type Key%20Structure :default "AnyKey"))
  (bind _colors (Variables|Default|GetColors))
  (:Pressed
    (for _array_element (Variables|Default|GetMaterialDynamic)
      (Rendering|Material|SetVectorParameterValue _array_element "Color" (Utilities|Array|Get(acopy) _colors (Variables|Default|GetColorIndex)) :!class /Script/Engine.MaterialInstanceDynamic))
    (if (> (Utilities|Array|Length _colors) (Variables|Default|GetColorIndex))
      (Math|Integer|IncrementInt (Variables|Default|GetColorIndex))
      (else
        (Variables|Default|SetColorIndex 0)))))

(fn ConstructionScript
  (bind _mesh (Variables|Default|GetMesh))
  (Utilities|Array|Resize (Variables|Default|GetMaterialDynamic) (Utilities|Array|Length _mesh))
  (for (_array_element _array_index) _mesh
    (bind _returnvalue (Rendering|Material|CreateDynamicMaterialInstance (Variables|/Script/Engine.StaticMeshActor|GetStaticMeshComponent _array_element) (Variables|Default|GetMaterialIndex) 0 :!class /Script/Engine.PrimitiveComponent))
    (Utilities|Array|SetArrayElem (Variables|Default|GetMaterialDynamic) _array_index _returnvalue)))