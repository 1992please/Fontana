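; BP_Door is an interactive door that opens and closes on an input action.
; A Box overlap enables input for the first player controller on entry and disables it on exit, without checking which actor overlaps.
; Each press alternates, via FlipFlop, between playing and reversing a timeline that drives the Door's relative yaw.
; The DoorDirection boolean selects between DoorRotation and DoorRotationNeg timelines for the swing.
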(event OnComponentBeginOverlap(Box)
  (params (OtherActor :type Actor%20Object%20Reference) (OtherComp :type Primitive%20Component%20Object%20Reference) (OtherBodyIndex :type Integer) (bFromSweep :type Boolean) (SweepResult :type Hit%20Result%20Structure%20%28by%20ref%29))
  (Input|EnableInput (Game|GetPlayerController 0)))

(event OnComponentEndOverlap(Box)
  (params (OtherActor :type Actor%20Object%20Reference) (OtherComp :type Primitive%20Component%20Object%20Reference) (OtherBodyIndex :type Integer))
  (Input|DisableInput (Game|GetPlayerController 0)))

(event EventBeginPlay)

(event EventActorBeginOverlap
  (params (OtherActor :type Actor%20Object%20Reference)))

(event EventTick
  (params (DeltaSeconds :type Float%20%28single-precision%29)))

(event Input|ActionEvents|InputActionDefualtAction
  (params (Key :type Key%20Structure :default "AnyKey"))
  (:Pressed
    (if (Variables|Default|GetDoorDirection)
      (Utilities|FlowControl|FlipFlop
        (:A
          (bind _doorrot (Timeline|DoorRotation Play)
            (:Update
              (Transformation|SetRelativeRotation (Variables|Default|GetDoor) (Math|Rotator|MakeRotator 0.0 0.0 _doorrot) false false))))
        (:B
          (Timeline|DoorRotation Reverse)))
      (else
        (Utilities|FlowControl|FlipFlop
          (:A
            (bind _doorrot_2 (Timeline|DoorRotationNeg Play)
              (:Update
                (Transformation|SetRelativeRotation (Variables|Default|GetDoor) (Math|Rotator|MakeRotator 0.0 0.0 _doorrot_2) false false))))
          (:B
            (Timeline|DoorRotationNeg Reverse)))))))

(fn ConstructionScript)