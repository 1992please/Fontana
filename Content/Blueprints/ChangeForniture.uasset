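; Blueprint actor that toggles between an old and a new set of furniture on the ChangeForniture input action.
; On BeginPlay it caches the direct child components under the OldParent and NewParent static meshes and enables input from player controller 0.
; A FlipFlop alternates which parent is visible, propagating to children, and sets cached mesh children to BlockAll for the shown set and NoCollision for the hidden one.
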(event EventBeginPlay
  (Variables|Default|SetNewForniture (Components|GetChildrenComponents (Variables|/Script/Engine.StaticMeshActor|GetStaticMeshComponent (Variables|Default|GetNewParent)) false))
  (Variables|Default|SetOldForniture (Components|GetChildrenComponents (Variables|/Script/Engine.StaticMeshActor|GetStaticMeshComponent (Variables|Default|GetOldParent)) false))
  (Input|EnableInput (Game|GetPlayerController 0)))

(event Input|ActionEvents|InputActionChangeForniture
  (params (Key :type Key%20Structure :default "AnyKey"))
  (bind _newparent (Variables|Default|GetNewParent))
  (bind _oldparent (Variables|Default|GetOldParent))
  (bind _staticmeshcomponent (Variables|/Script/Engine.StaticMeshActor|GetStaticMeshComponent _newparent))
  (bind _staticmeshcomponent_2 (Variables|/Script/Engine.StaticMeshActor|GetStaticMeshComponent _oldparent))
  (:Pressed
    (Utilities|FlowControl|FlipFlop
      (:A
        (Rendering|SetVisibility _staticmeshcomponent_2 false true)
        (Rendering|SetVisibility _staticmeshcomponent true true)
        (for _array_element (Variables|Default|GetOldForniture)
          (bind _asmesh_component (Utilities|Casting|CastToMeshComponent _array_element))
          (Collision|SetCollisionProfileName _asmesh_component "NoCollision" :!class /Script/Engine.PrimitiveComponent))
        (for _array_element_2 (Variables|Default|GetNewForniture)
          (bind _asmesh_component_2 (Utilities|Casting|CastToMeshComponent _array_element_2))
          (Collision|SetCollisionProfileName _asmesh_component_2 "BlockAll" :!class /Script/Engine.PrimitiveComponent)))
      (:B
        (Rendering|SetVisibility _staticmeshcomponent_2 true true)
        (Rendering|SetVisibility _staticmeshcomponent false true)
        (for _array_element_3 (Variables|Default|GetOldForniture)
          (bind _asmesh_component_3 (Utilities|Casting|CastToMeshComponent _array_element_3))
          (Collision|SetCollisionProfileName _asmesh_component_3 "BlockAll" :!class /Script/Engine.PrimitiveComponent))
        (for _array_element_4 (Variables|Default|GetNewForniture)
          (bind _asmesh_component_4 (Utilities|Casting|CastToMeshComponent _array_element_4))
          (Collision|SetCollisionProfileName _asmesh_component_4 "NoCollision" :!class /Script/Engine.PrimitiveComponent))))))

(fn ConstructionScript)