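; Actor that lets the player recolor one material slot on its mesh by pressing ChangeColors while inside a trigger box.
; The construction script creates a dynamic material instance for every mesh slot, and box overlaps toggle player 0's input on the actor.
; Each press applies the current Colors entry to the MaterialIndex slot's Color parameter, then advances, with the index reaching the array length before resetting.
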(event OnComponentBeginOverlap(Box)
  (params (OtherActor :type Actor%20Object%20Reference) (OtherComp :type Primitive%20Component%20Object%20Reference) (OtherBodyIndex :type Integer) (bFromSweep :type Boolean) (SweepResult :type Hit%20Result%20Structure%20%28by%20ref%29))
  (Input|EnableInput (Game|GetPlayerController 0)))

(event OnComponentEndOverlap(Box)
  (params (OtherActor :type Actor%20Object%20Reference) (OtherComp :type Primitive%20Component%20Object%20Reference) (OtherBodyIndex :type Integer))
  (Input|DisableInput (Game|GetPlayerController 0)))

(event EventBeginPlay)

(event Collision|EventActorBeginOverlap
  (params (OtherActor :type Actor%20Object%20Reference)))

(event EventTick
  (params (DeltaSeconds :type Float%20%28single-precision%29)))

(event Input|ActionEvents|InputActionChangeColors
  (params (Key :type Key%20Structure :default "AnyKey"))
  (bind _colors (Variables|Default|GetColors))
  (:Pressed
    (Rendering|Material|SetVectorParameterValue (Utilities|Array|Get(acopy) (Variables|Default|GetMaterialDynamic) (Variables|Default|GetMaterialIndex)) "Color" (Utilities|Array|Get(acopy) _colors (Variables|Default|GetColorIndex)) :!class /Script/Engine.MaterialInstanceDynamic)
    (if (> (Utilities|Array|Length _colors) (Variables|Default|GetColorIndex))
      (Math|Integer|IncrementInt (Variables|Default|GetColorIndex))
      (else
        (Variables|Default|SetColorIndex 0)))))

(fn ConstructionScript
  (bind _materialdynamic (Variables|Default|GetMaterialDynamic))
  (bind _mesh (Variables|Default|GetMesh))
  (bind _staticmeshcomponent (Variables|/Script/Engine.StaticMeshActor|GetStaticMeshComponent _mesh))
  (bind _returnvalue (Rendering|Material|GetNumMaterials _staticmeshcomponent))
  (Utilities|Array|Resize _materialdynamic _returnvalue)
  (for _index (range 0 (- _returnvalue 1))
    (bind _returnvalue_2 (Rendering|Material|CreateDynamicMaterialInstance _staticmeshcomponent _index 0 :!class /Script/Engine.PrimitiveComponent))
    (Utilities|Array|SetArrayElem _materialdynamic _index _returnvalue_2)))